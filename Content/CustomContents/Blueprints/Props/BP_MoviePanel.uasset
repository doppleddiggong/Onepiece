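; BP_MoviePanel is a prop that plays a movie on its material through a MediaPlayer.
; RecvOnMovie filters by group, then either starts playback with a white tint and media texture, or closes the player and blacks out the panel unless OneShot is set.
; The BroadcastManager binding and dynamic material setup sit in unconnected nodes, and BeginPlay is empty, so this graph never wires up either.
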(event `self.ReceiveBeginPlay`)

(event `RecvOnMovie`
  (params (Group :type Integer) (State :type Boolean))
  (if (== Group (`self.Group`))
    (if State
      (if (not (`MediaPlayer.IsPlaying` (`self.MediaPlayer`)))
        (`MediaPlayer.OpenSource` (`self.MediaPlayer`) (`self.Media Source`))
        (`MediaPlayer.Play` (`self.MediaPlayer`))
        (`MaterialInstanceDynamic.SetVectorParameterValue` (`self.MediaMaterial`) "Color" (struct :`R` 1.0 :`G` 1.0 :`B` 1.0 :`A` 1.0))
        (`MaterialInstanceDynamic.SetTextureParameterValue` (`self.MediaMaterial`) "MediaTexture" (`self.MediaTexture`)))
      (elif (not (`self.OneShot`))
        (`MediaPlayer.Rewind` (`self.MediaPlayer`))
        (`MediaPlayer.Close` (`self.MediaPlayer`))
        (`MaterialInstanceDynamic.SetVectorParameterValue` (`self.MediaMaterial`) "Color" (struct :`A` 1.0))))))

(fn `UserConstructionScript`)