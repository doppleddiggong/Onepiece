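; BP_BroadcastTrigger_Door is an interactable trigger that broadcasts a door open-state message in multiplayer games.
; On activation it checks IsMultiPlay, then sends its door index and Open flag, with itself as instigator, through the NetworkBroadcastActor's SendDoorMessage.
; In single player it only prints that the element is inactive, and a missing broadcast actor prints a failure message.
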(event `self.OnActivate`
  (bind _returnvalue (`NetworkBroadcastLibrary.GetNetworkBroadcastActor`))
  (bind _returnvalue_2 (`LingoGameHelper.IsMultiPlay` self))
  (if _returnvalue_2
    (`/Engine/EditorBlueprintResources/StandardMacros.IsValid` _returnvalue
      (:`Is Valid`
        (`NetworkBroadcastActor.SendDoorMessage` _returnvalue (`self.In Door Index`) (`self.Open`) self)
        (`KismetSystemLibrary.PrintString` "멀티 플레이 요소 발동"))
      (:`Is Not Valid`
        (`KismetSystemLibrary.PrintString` "Find NetworkBroadcastActor Fail")))
    (else
      (`KismetSystemLibrary.PrintString` "싱글 플레이 미발동 요소"))))

(fn `UserConstructionScript`)