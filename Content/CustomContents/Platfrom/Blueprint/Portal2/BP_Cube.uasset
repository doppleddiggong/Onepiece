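; Portal cube that can pass between BP_Portal1 and BP_Portal2, showing a duplicate at the exit during transit.
; While duplication is active, Tick mirrors the body's entry-relative transform onto the copy attached to the exit door.
; Deactivation hides the copy and snaps the body to it unless a portal's grab flag is set.
; Velocity functions teleport the cube to the other portal, redirecting its speed along the exit arrow or through portal-relative direction.
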(event `self.ReceiveBeginPlay`
  (bind _returnvalue (`GameplayStatics.GetActorOfClass` "/Game/CustomContents/Portal/BP/BP_Portal1.BP_Portal1_C"))
  (set `self.Portal1` _returnvalue)
  (bind _returnvalue_2 (`GameplayStatics.GetActorOfClass` "/Game/CustomContents/Portal/BP/BP_Portal2.BP_Portal2_C"))
  (set `self.Portal2` _returnvalue_2))

(event `self.ReceiveTick`
  (params (DeltaSeconds :type "Float (single-precision)"))
  (bind _entry_door (`self.Entry Door`))
  (bind _staticmesh_body (`self.StaticMesh_Body`))
  (bind (_returnvalue_location _returnvalue_rotation) (`KismetMathLibrary.BreakTransform` (`KismetMathLibrary.MakeRelativeTransform` (`SceneComponent.K2_GetComponentToWorld` _staticmesh_body) (`SceneComponent.K2_GetComponentToWorld` _entry_door))))
  ;[0.05286 0.159 1] 복제본 위치 변경하기
  (if (`self.DuplicateActivated`)
    (`/Engine/EditorBlueprintResources/StandardMacros.IsValid` _entry_door
      (:`Is Valid`
        (`SceneComponent.K2_SetRelativeTransform` (`self.Copy`) (`KismetMathLibrary.MakeTransform` (`KismetMathLibrary.RotateAngleAxis` _returnvalue_location 180.0 (`SceneComponent.GetUpVector` _entry_door)) (`KismetMathLibrary.ComposeRotators` _returnvalue_rotation (struct :`Yaw` 180.0)) (`SceneComponent.K2_GetComponentScale` _staticmesh_body)) false false)))))

(event `/Game/CustomContents/Portal/BP/BPI_PortalJumper.ActivateDuplicate`
  (params (EntryDoor :type "SceneComponent Object Reference") (ExitDoor :type "SceneComponent Object Reference"))
  (bind _portal1 (`self.Portal1`))
  (bind _portal2 (`self.Portal2`))
  (set `self.Entry Door` EntryDoor)
  (set `self.Exit Door` ExitDoor)
  (set `self.WeaponCP` (`self.GetComponentByClass` (`GameplayStatics.GetPlayerCharacter` 0) "/Game/CustomContents/Portal/BP/BP_WeaponComponent.BP_WeaponComponent_C"))
  ;[0.05286 0.159 1] COPY 활성화
  (`SceneComponent.K2_DetachFromComponent` (`self.Copy`) "KeepWorld" "KeepWorld" "KeepWorld" true)
  (set `self.DuplicateActivated` true)
  (`self.SetHiddenInGame_Copy` false)
  (`SceneComponent.SetRelativeScale3D` (`self.StaticMesh_Symbol_Copy`) (0.75 0.75 0.75))
  (`SceneComponent.SetRelativeScale3D` (`self.StaticMesh_Cover_Copy`) (0.75 0.75 0.75))
  (`SceneComponent.SetRelativeScale3D` (`self.StaticMesh_Body_Copy`) (0.75 0.75 0.75))
  (`SceneComponent.K2_AttachToComponent` (`self.Copy`) (`self.Exit Door`) "None" "KeepWorld" "KeepWorld" "KeepWorld" true)
  (`/Engine/EditorBlueprintResources/StandardMacros.IsValid` _portal1
    (:`Is Valid`
      (set `/Game/CustomContents/Portal/BP/BP_Portal1.PlayerGrabCube1` false _portal1)
      (`/Engine/EditorBlueprintResources/StandardMacros.IsValid` _portal2
        (:`Is Valid`
          (set `/Game/CustomContents/Portal/BP/BP_Portal2.PlayerGrabCube2` false _portal2))))))

(event `self.ActivateDisolve`
  (`CommonFunctionLibrary.PlayLocationSound` self "/Game/CustomContents/Platfrom/Sound/Cue/Disolve_Cue.Disolve_Cue" 0.05))

(event `/Game/CustomContents/Portal/BP/BPI_PortalJumper.DeactivateDuplicate`
  (bind _portal2 (`self.Portal2`))
  (bind _portal1 (`self.Portal1`))
  (bind (_returnvalue_location _returnvalue_rotation) (`KismetMathLibrary.BreakTransform` (`SceneComponent.K2_GetComponentToWorld` (`self.Copy`))))
  ;[0.05286 0.159 1] Copy 비활성화
  (`self.SetHiddenInGame_Copy` true)
  (if (`self.DuplicateActivated`)
    (set `self.DuplicateActivated` false)
    (`self.SetHiddenInGame_Copy` true)
    (bind _returnvalue (`GameplayStatics.GetActorOfClass` "/Game/CustomContents/Portal/BP/BP_Portal1.BP_Portal1_C"))
    (set `self.Portal1` _returnvalue)
    (bind _returnvalue_2 (`GameplayStatics.GetActorOfClass` "/Game/CustomContents/Portal/BP/BP_Portal2.BP_Portal2_C"))
    (set `self.Portal2` _returnvalue_2)
    (`/Engine/EditorBlueprintResources/StandardMacros.IsValid` _portal1
      (:`Is Valid`
        (`/Engine/EditorBlueprintResources/StandardMacros.IsValid` _portal2
          (:`Is Valid`
            (if (not (or (`/Game/CustomContents/Portal/BP/BP_Portal1.PlayerGrabCube1` _portal1) (`/Game/CustomContents/Portal/BP/BP_Portal2.PlayerGrabCube2` _portal2)))
              (`SceneComponent.K2_SetWorldTransform` (`self.StaticMesh_Body`) (`KismetMathLibrary.MakeTransform` _returnvalue_location _returnvalue_rotation (`SceneComponent.K2_GetComponentScale` (`self.StaticMesh_Body`))) false false))
            (`self.SetHiddenInGame_Original` false)
            (`self.SetHiddenInGame_Copy` true)
            (`SceneComponent.K2_AttachToComponent` (`self.Copy`) (`self.StaticMesh_Body`) "None" "KeepRelative" "KeepRelative" "KeepRelative" true)
            (set `/Game/CustomContents/Portal/BP/BP_Portal1.PlayerGrabCube1` false (`self.Portal1`))
            (set `/Game/CustomContents/Portal/BP/BP_Portal2.PlayerGrabCube2` false (`self.Portal2`))
            (set `self.DuplicateActivated` false)))))))

(fn `InitScale`
  (`self.SetActorScale3D` self (`self.InitSclaeValue`)))

(fn `SetCubeVelocity2`
  (bind _returnvalue (`SceneComponent.GetComponentVelocity` (`self.StaticMesh_Body`)))
  (`|ExecutionSequence`
    (:`then_0`
      ; 입구 들어갈때 속도
      (set `self.V_in_2` _returnvalue)
      (bind _output_get (set `self.Speed` (`KismetMathLibrary.VSize` _returnvalue)))
      (if (> _output_get 4096.0)
        (set `self.Speed` 4095.0)
        (else
          (set `self.Speed` (`self.Speed`))))
      (bind _returnvalue_2 (`GameplayStatics.GetActorOfClass` "/Game/CustomContents/Portal/BP/BP_Portal2.BP_Portal2_C"))
      (set `self.Portal2` _returnvalue_2)
      (bind _returnvalue_3 (`GameplayStatics.GetActorOfClass` "/Game/CustomContents/Portal/BP/BP_Portal1.BP_Portal1_C"))
      (set `self.Portal1` _returnvalue_3))
    (:`then_1`
      ; 출구 기준 월드로 변환
      (set `self.Vector Out` (* (`KismetMathLibrary.TransformDirection` (`SceneComponent.K2_GetComponentToWorld` (`Actor.RootComponent` (`self.Portal2`))) (`KismetMathLibrary.Normal` (`KismetMathLibrary.InverseTransformDirection` (`SceneComponent.K2_GetComponentToWorld` (`Actor.RootComponent` (`self.Portal1`))) (`self.V_in_2`)))) (`self.Speed`))))
    (:`then_2`
      ; 위치변경
      (`self.K2_SetActorLocationAndRotation` (`self.K2_GetActorLocation` (`self.Portal2`)) (struct) false true)
      (`PrimitiveComponent.SetPhysicsLinearVelocity` (`self.StaticMesh_Body`) (`self.Vector Out`) false "None"))))

(fn `SetCubeVelocity_p1`
  (bind _portal2 (`self.Portal2`))
  (bind _portal2_2 (`self.Portal2`))
  (`|ExecutionSequence`
    (:`then_0`
      ; 입구 들어갈때 속도
      (set `self.Speed` (`KismetMathLibrary.VSize` (`SceneComponent.GetComponentVelocity` (`self.StaticMesh_Body`))))
      (`/Engine/EditorBlueprintResources/StandardMacros.IsValid` _portal2
        (:`Is Valid`
          (set `self.Vector Out` (* (`KismetMathLibrary.Normal` (`SceneComponent.GetForwardVector` (`/Game/CustomContents/Portal/BP/BP_Portal2.Arrow` _portal2))) (`self.Speed`))))
        (:`Is Not Valid`
          (bind _returnvalue (`GameplayStatics.GetActorOfClass` "/Game/CustomContents/Portal/BP/BP_Portal2.BP_Portal2_C"))
          (bind _output_get (set `self.Portal2` _returnvalue))
          (set `self.Vector Out` (* (`SceneComponent.GetForwardVector` (`/Game/CustomContents/Portal/BP/BP_Portal2.Arrow` _output_get)) (`self.Speed`))))))
    (:`then_1`
      ; 위치변경
      (`self.K2_SetActorLocationAndRotation` (+ (`self.K2_GetActorLocation` _portal2_2) (* (`SceneComponent.GetForwardVector` (`/Game/CustomContents/Portal/BP/BP_Portal2.Arrow` _portal2_2)) 100.0)) (struct) false true)
      (`PrimitiveComponent.SetPhysicsLinearVelocity` (`self.StaticMesh_Body`) (`self.Vector Out`) false "None"))))

(fn `SetCubeVelocity_p2`
  (bind _portal1 (`self.Portal1`))
  (bind _portal1_2 (`self.Portal1`))
  (`|ExecutionSequence`
    (:`then_0`
      ; 입구 들어갈때 속도
      (set `self.Speed` (`KismetMathLibrary.VSize` (`SceneComponent.GetComponentVelocity` (`self.StaticMesh_Body`))))
      (`/Engine/EditorBlueprintResources/StandardMacros.IsValid` _portal1
        (:`Is Valid`
          (set `self.Vector Out` (* (`KismetMathLibrary.Normal` (`SceneComponent.GetForwardVector` (`/Game/CustomContents/Portal/BP/BP_Portal1.Arrow` _portal1))) (`self.Speed`))))
        (:`Is Not Valid`
          (bind _returnvalue (`GameplayStatics.GetActorOfClass` "/Game/CustomContents/Portal/BP/BP_Portal1.BP_Portal1_C"))
          (bind _output_get (set `self.Portal1` _returnvalue))
          (set `self.Vector Out` (* (`SceneComponent.GetForwardVector` (`/Game/CustomContents/Portal/BP/BP_Portal1.Arrow` _output_get)) (`self.Speed`))))))
    (:`then_1`
      ; 위치변경
      (`PrimitiveComponent.SetCollisionResponseToChannel` (`self.StaticMesh_Body`) "ECC_GameTraceChannel4" "ECR_Ignore")
      (`self.K2_SetActorLocationAndRotation` (+ (`self.K2_GetActorLocation` _portal1_2) (* (`SceneComponent.GetForwardVector` (`/Game/CustomContents/Portal/BP/BP_Portal1.Arrow` _portal1_2)) 100.0)) (struct) false true)
      (`PrimitiveComponent.SetPhysicsLinearVelocity` (`self.StaticMesh_Body`) (`self.Vector Out`) false "None")
      (`PrimitiveComponent.SetCollisionResponseToChannel` (`self.StaticMesh_Body`) "ECC_GameTraceChannel4" "ECR_Overlap"))))

(fn `SetHiddenInGame_Copy`
  (params (NewHidden :type Boolean))
  (`|ExecutionSequence`
    (:`then_0`
      (`SceneComponent.SetHiddenInGame` (`self.StaticMesh_Body_Copy`) NewHidden false))
    (:`then_1`
      (`SceneComponent.SetHiddenInGame` (`self.StaticMesh_Cover_Copy`) NewHidden false))
    (:`then_2`
      (`SceneComponent.SetHiddenInGame` (`self.StaticMesh_Symbol_Copy`) NewHidden false))))

(fn `SetHiddenInGame_Original`
  (params (NewHidden :type Boolean))
  (`|ExecutionSequence`
    (:`then_0`
      (`SceneComponent.SetHiddenInGame` (`self.StaticMesh_Body`) NewHidden false))
    (:`then_1`
      (`SceneComponent.SetHiddenInGame` (`self.StaticMesh_Cover`) NewHidden false))
    (:`then_2`
      (`SceneComponent.SetHiddenInGame` (`self.StaticMesh_Symbol`) NewHidden false))))

(fn `StoreCubeVelocity`
  (set `self.CubeVelocity` (`SceneComponent.GetComponentVelocity` (`self.StaticMesh_Body`))))

(fn `UserConstructionScript`)