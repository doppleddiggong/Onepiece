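; Portal 2 style cube button that shows its on or off state through emissive color and animation.
; On BeginPlay it creates a dynamic material on the switch body, caches the ABP_CubeButton anim instance and binds to switch-state changes.
; Each change sets the active or inactive color, forwards the state to the Animation Blueprint and prints a debug message.
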(event `self.ReceiveBeginPlay`
  (`self.InitSwitch`)
  (add `self.OnChangeSwitchState` (delegate `SwitchChange`)))

(event `SwitchChange` :!signature `self.OnChangeSwitchState`
  (params (bIsActive :type Boolean))
  (if bIsActive
    (`self.SetActivate` true)
    (`KismetSystemLibrary.PrintString` "Click On")
    (else
      (`self.SetActivate` false)
      (`KismetSystemLibrary.PrintString` "Click Off"))))

(fn `InitSwitch`
  (bind _returnvalue (`PrimitiveComponent.CreateDynamicMaterialInstance` (`self.SwitchBody`) 0 (`PrimitiveComponent.GetMaterial` (`self.SwitchBody`) 0) "None"))
  (bind _output_get (set `self.EmisiveMaterial` _returnvalue))
  (`MaterialInstanceDynamic.SetVectorParameterValue` _output_get (`self.ColorParam`) (`self.DeactivateColor`))
  (bind _asabp_cube_button (cast `/Game/CustomContents/Platfrom/Blueprint/Portal2/ABP_CubeButton` (`SkeletalMeshComponent.GetAnimInstance` (`self.SwitchBody`))))
  (set `self.AnimBlueprint` _asabp_cube_button))

(fn `SetActivate`
  (params (State :type Boolean))
  (`MaterialInstanceDynamic.SetVectorParameterValue` (`self.EmisiveMaterial`) (`self.EmisiveParam`) (`KismetMathLibrary.SelectColor` (`self.ActivateColor`) (`self.DeactivateColor`) State))
  (`TweenAnimInstance.ChangeState` (`self.AnimBlueprint`) State))

(fn `UserConstructionScript`)