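; BP_Pedestal_Button is a Portal 2-style pedestal button that plays a press animation when OnClickSwitch fires.
; On BeginPlay it caches its ABP_Pedestal_Button anim instance, whose ChangeState drives the press, with a one-second delay blocking repeat clicks.
; Collision overlaps with PlayerActor toggle a DetectTarget flag, which this file never reads.
; Spawning is unfinished: the OneSpawn branch only checks SpawnedActor validity, and ActiveSwitch just animates and prints debug text.
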(event `self.ReceiveBeginPlay`
  ; Begin
  (`self.InitButton`))

(event `self.Collision.OnComponentBeginOverlap`
  (params (OverlappedComponent :type "PrimitiveComponent Object Reference") (OtherActor :type "Actor Object Reference") (OtherComp :type "PrimitiveComponent Object Reference") (OtherBodyIndex :type Integer) (bFromSweep :type Boolean) (SweepResult :type "HitResult Structure (by ref)"))
  ; Collision
  (cast `PlayerActor` OtherActor)
  (set `self.DetectTarget` true))

(event `self.Collision.OnComponentEndOverlap`
  (params (OverlappedComponent :type "PrimitiveComponent Object Reference") (OtherActor :type "Actor Object Reference") (OtherComp :type "PrimitiveComponent Object Reference") (OtherBodyIndex :type Integer))
  ; Collision
  (cast `PlayerActor` OtherActor)
  (set `self.DetectTarget` false))

(event `OnClickSwitch`
  ; OnClickSwitch
  (if (not (`self.Input Delay`))
    (set `self.Input Delay` true)
    (`/Game/CustomContents/Platfrom/Blueprint/Portal2/ABP_Pedestal_Button.ChangeState` (`self.AnimBlueprint`) true)
    (`|ExecutionSequence`
      (:`then_0`
        (`KismetSystemLibrary.Delay` 1.0)
        (set `self.Input Delay` false))
      (:`then_1`
        (if (`self.OneSpawn`)
          (`/Engine/EditorBlueprintResources/StandardMacros.IsValid` (`self.SpawnedActor`)))))))

(fn `ActiveSwitch`
  (`/Game/CustomContents/Platfrom/Blueprint/Portal2/ABP_Pedestal_Button.ChangeState` (`self.AnimBlueprint`) true)
  (if (`self.OneSpawn`)
    (`KismetSystemLibrary.PrintString` "Spawn TRUE")
    (else
      (`KismetSystemLibrary.PrintString` "Spawn FALSE"))))

(fn `InitButton`
  (bind _asabp_pedestal_button (cast `/Game/CustomContents/Platfrom/Blueprint/Portal2/ABP_Pedestal_Button` (`SkeletalMeshComponent.GetAnimInstance` (`self.Switch Body`))))
  (set `self.AnimBlueprint` _asabp_pedestal_button))

(fn `UserConstructionScript`)