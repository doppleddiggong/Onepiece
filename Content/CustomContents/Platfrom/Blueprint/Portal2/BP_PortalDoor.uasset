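; BP_PortalDoor is a two-panel sliding door that opens and closes in response to broadcast messages.
; On BeginPlay it binds to the BroadcastManager and matches each message against its open and close messages.
; A timeline, eased out cubically on update, lerps both meshes between relative zero and their open offsets.
; Closing plays the timeline in reverse and is skipped when OneShot is set.
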(event `self.ReceiveBeginPlay`
  (add `BroadcastManager.OnMessage` (subsystem `BroadcastManager`) (delegate `RecvOnMessage`)))

(event `RecvOnMessage`
  (params (Msg :type String))
  (bind _msgtype (`self.RecvMessageType` Msg))
  (switch `int` _msgtype
    (:`0`
      (`self.OpenDoor`))
    (:`1`
      (`self.CloseDoor`))))

(event `OpenDoor`
  (bind (_direction _alpha) (`Timeline|TL_Door` :!via `PlayFromStart` :!label _label)
    (:`Update`
      (`self.UpdateDoor` (`EaseFunctionLibrary.EaseAlphaCustom` _alpha "EaseOutCubic")))))

(event `CloseDoor`
  (if (not (`self.OneShot`))
    (goto _label :!via `ReverseFromEnd`)))

(fn `RecvMessageType`
  (params (Msg :type String))
  (returns (MsgType :type Integer))
  (if (`KismetStringLibrary.EqualEqual_StrStr` Msg (`self.OpenMessage`))
    (return 0)
    (elif (`KismetStringLibrary.EqualEqual_StrStr` Msg (`self.CloseMessage`))
      (return 1)
      (else
        (return -1)))))

(fn `UpdateDoor`
  (params (Alpha :type "Float (double-precision)"))
  (locals (InAlpha :type "Float (double-precision)"))
  (set `local.InAlpha` Alpha)
  (`|ExecutionSequence`
    (:`then_0`
      (`SceneComponent.K2_SetRelativeLocation` (`self.SM_Right`) (`KismetMathLibrary.VLerp` (0.0 0.0 0.0) (`self.Right_Open`) (`local.InAlpha`)) false false))
    (:`then_1`
      (`SceneComponent.K2_SetRelativeLocation` (`self.SM_Left`) (`KismetMathLibrary.VLerp` (0.0 0.0 0.0) (`self.Left_Open`) (`local.InAlpha`)) false false))))

(fn `UserConstructionScript`)